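; VR pawn for a painting app that moves by left-grip dragging and orbits with the left thumbstick, caching its child-actor color picker on BeginPlay.
; Tick tracks left-controller position and rotation deltas; while grip is held, the root moves against hand motion, scaled by inverse delta time.
; Thumbstick Y rotates the location around world Z, yaws toward Center and passes that yaw to a pawn-update delegate.
; Zoom and the rotation delta are unused here.
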(event `self.ReceiveBeginPlay`
  (`HeadMountedDisplayFunctionLibrary.SetTrackingOrigin` "Floor")
  (bind _asbp_color_picker (cast `/Game/BP_ColorPicker` (`ChildActorComponent.ChildActor` (`self.W_Colorpicker`))))
  (set `self.Cpicker` _asbp_color_picker))

(event `self.ReceiveTick`
  (params (DeltaSeconds :type "Float (single-precision)"))
  (`self.GetLinearVel`)
  (`self.GetAngularVel`)
  (if (`self.bMove`)
    (`SceneComponent.K2_AddWorldOffset` (`self.RootComponent`) (* (/ (`self.NewLoc`) (`GameplayStatics.GetWorldDeltaSeconds`)) -0.0155) false false)))

(event `Key|MotionController_Left_Grip1`
  (params (Key :type "Key Structure"))
  (:`Pressed`
    (set `self.bMove` true))
  (:`Released`
    (set `self.bMove` false)))

(event `InputAxisKey|MotionController_Left_Thumbstick_Y`
  (params (AxisValue :type "Float (single-precision)"))
  (bind (_returnvalue_roll _returnvalue_pitch _returnvalue_yaw) (`KismetMathLibrary.BreakRotator` (`KismetMathLibrary.FindLookAtRotation` (`SceneComponent.K2_GetComponentLocation` (`self.RootComponent`)) (`SceneComponent.K2_GetComponentLocation` (`self.Center`)))))
  (if (!= AxisValue 0.0)
    (`KismetSystemLibrary.PrintString` (`KismetStringLibrary.Conv_RotatorToString` (struct)))
    (`self.K2_SetActorLocation` (`KismetMathLibrary.RotateAngleAxis` (+ (`self.K2_GetActorLocation`) (0.0 0.0 0.0)) AxisValue (0.0 0.0 1.0)))
    (`SceneComponent.K2_SetWorldRotation` (`self.RootComponent`) (`KismetMathLibrary.MakeRotator` 0.0 0.0 _returnvalue_yaw) false false)
    (`self.FPawnUpdateDelegate` (`KismetMathLibrary.MakeRotator` 0.0 0.0 _returnvalue_yaw))))

(fn `GetAngularVel`
  (bind _returnvalue (`SceneComponent.K2_GetComponentRotation` (`self.MC_Left`)))
  (bind _output_get (set `self.NewRot` (`KismetMathLibrary.Conv_VectorToRotator` (- (`KismetMathLibrary.Conv_RotatorToVector` _returnvalue) (`KismetMathLibrary.Conv_RotatorToVector` (`self.PrevRot`))))))
  (set `self.PrevRot` _returnvalue))

(fn `GetLinearVel`
  (bind _returnvalue (`SceneComponent.K2_GetComponentLocation` (`self.MC_Left`)))
  (set `self.NewLoc` (- _returnvalue (`self.prevLoc`)))
  (set `self.prevLoc` _returnvalue))

(fn `UserConstructionScript`)

(fn `Zoom`
  (params (ZoomSpeed :type "Float (double-precision)"))
  (`self.K2_AddActorWorldOffset` (* (`SceneComponent.GetForwardVector` (`self.RootComponent`)) (`KismetMathLibrary.Conv_DoubleToVector` ZoomSpeed) (-1.0 -1.0 -1.0))))