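; Color picker actor with a hue bar and a saturation/value plate, operated by actors overlapping either component.
; An overlap line-traces that component from the overlapping actor and reads the hit's collision UV.
; Colorbar UV sets Hue, which Tick pushes to the plate's dynamic saturation-mask material.
; Plate UV supplies saturation and value, combined with Hue into SelectedColor and broadcast through the color update delegate.
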(event `self.ReceiveBeginPlay`
  (bind _returnvalue (`PrimitiveComponent.CreateDynamicMaterialInstance` (`self.SaturationPlate`) 0 "/Game/HDAssets/MI_SaturationMask.MI_SaturationMask"))
  (bind _output_get (set `self.DynamicMatInstance` _returnvalue))
  (`PrimitiveComponent.SetMaterial` (`self.SaturationPlate`) 0 _output_get))

(event `self.ReceiveTick`
  (params (DeltaSeconds :type "Float (single-precision)"))
  (`MaterialInstanceDynamic.SetVectorParameterValue` (stale `self.ReceiveBeginPlay` _output_get) "HueValue" (`self.Hue`)))

(event `self.Colorbar.OnComponentBeginOverlap`
  (params (OverlappedComponent :type "PrimitiveComponent Object Reference") (OtherActor :type "Actor Object Reference") (OtherComp :type "PrimitiveComponent Object Reference") (OtherBodyIndex :type Integer) (bFromSweep :type Boolean) (SweepResult :type "HitResult Structure (by ref)"))
  (bind (_h _s _v _a) (`KismetMathLibrary.RGBToHSV` (`self.Hue`)))
  (bind (_hitlocation _hitnormal _bonename _outhit _returnvalue) (`PrimitiveComponent.K2_LineTraceComponent` (`self.Colorbar`) (`self.K2_GetActorLocation` OtherActor) (* (`self.GetActorForwardVector` OtherActor) 1000) true false))
  (if _returnvalue
    (bind _uv (`GameplayStatics.FindCollisionUV` _outhit))
    (set `self.Hue` (`KismetMathLibrary.HSVToRGB` (`KismetMathLibrary.MapRangeClamped` (`.Y` (`KismetMathLibrary.BreakVector2D` _uv)) 0.0 1.0 0.0 360.0) _s _v _a))
    (`KismetSystemLibrary.PrintString` (`KismetStringLibrary.Concat_StrStr` "X:" (`KismetStringLibrary.Conv_DoubleToString` (`KismetMathLibrary.BreakVector2D` _uv))))
    (`KismetSystemLibrary.PrintString` (`KismetStringLibrary.Concat_StrStr` "Y:" (`KismetStringLibrary.Conv_DoubleToString` (`.Y` (`KismetMathLibrary.BreakVector2D` _uv)))) true true (struct :`R` 1.0 :`B` 0.786245 :`A` 1.0))))

(event `self.SaturationPlate.OnComponentBeginOverlap`
  (params (OverlappedComponent :type "PrimitiveComponent Object Reference") (OtherActor :type "Actor Object Reference") (OtherComp :type "PrimitiveComponent Object Reference") (OtherBodyIndex :type Integer) (bFromSweep :type Boolean) (SweepResult :type "HitResult Structure (by ref)"))
  (bind (_h _s _v _a) (`KismetMathLibrary.RGBToHSV` (`self.Hue`)))
  (bind (_hitlocation _hitnormal _bonename _outhit) (`PrimitiveComponent.K2_LineTraceComponent` (`self.SaturationPlate`) (`self.K2_GetActorLocation` OtherActor) (* (`self.GetActorForwardVector` OtherActor) 1000) true false))
  (bind _uv (`GameplayStatics.FindCollisionUV` _outhit))
  (bind _output_get (set `self.SelectedColor` (`KismetMathLibrary.HSVToRGB` _h (`KismetMathLibrary.BreakVector2D` _uv) (`.Y` (`KismetMathLibrary.BreakVector2D` _uv)) _a)))
  (`self.FColorUpdateDelegate` _output_get))

(fn `UserConstructionScript`)